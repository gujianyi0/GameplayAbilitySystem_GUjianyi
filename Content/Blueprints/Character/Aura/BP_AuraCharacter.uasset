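; BP_AuraCharacter is the Blueprint for the Aura character, adding facing, shock-loop state and fading of overlapped actors.
; UpdateFacingTarget feeds a location to Motion Warping as the FacingTarget warp target, and SetinShockLoop stores the InShockLoop flag.
; A Box component's begin and end overlaps send fade-out and fade-in messages to actors implementing BI_FadeInterface, leaving the fade itself to those actors.
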(event `CombatInterface.UpdateFacingTarget`
  (params (Target :type "Vector Structure (by ref)"))
  (`MotionWarpingComponent.AddOrUpdateWarpTargetFromLocation` (`self.MotionWarping`) "FacingTarget" Target))

(event `CombatInterface.SetInShockLoop`
  (params (bInLoop :type Boolean))
  (set `self.InShockLoop` bInLoop))

(event `self.Box.OnComponentBeginOverlap`
  (params (OverlappedComponent :type "PrimitiveComponent Object Reference") (OtherActor :type "Actor Object Reference") (OtherComp :type "PrimitiveComponent Object Reference") (OtherBodyIndex :type Integer) (bFromSweep :type Boolean) (SweepResult :type "HitResult Structure (by ref)"))
  (if (`KismetSystemLibrary.DoesImplementInterface` OtherActor "/Game/Blueprints/Actor/FadeActor/BI_FadeInterface.BI_FadeInterface_C")
    (message `/Game/Blueprints/Actor/FadeActor/BI_FadeInterface.FadeOut` OtherActor)))

(event `self.Box.OnComponentEndOverlap`
  (params (OverlappedComponent :type "PrimitiveComponent Object Reference") (OtherActor :type "Actor Object Reference") (OtherComp :type "PrimitiveComponent Object Reference") (OtherBodyIndex :type Integer))
  (if (`KismetSystemLibrary.DoesImplementInterface` OtherActor "/Game/Blueprints/Actor/FadeActor/BI_FadeInterface.BI_FadeInterface_C")
    (message `/Game/Blueprints/Actor/FadeActor/BI_FadeInterface.FadeIn` OtherActor)))

(fn `UserConstructionScript`)